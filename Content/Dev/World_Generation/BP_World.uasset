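; World actor that generates procedural terrain tiles around the player as they move.
; A one-second looping timer queues nearby grid tiles and starts async generation of the closest ungenerated one, or draws it once data is ready.
; An unused Blueprint generator remains, layering Perlin noise for height.
; It computes normals and tangents on a grid with a one-vertex border, then trims it so section edges shade seamlessly.
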(event `self.ReceiveBeginPlay`
  (`self.PlayerSpawnTiles`)
  (`KismetSystemLibrary.K2_SetTimer` null "PlayerSpawnTiles" 1.0 true))

(event `PlayerSpawnTiles`
  (bind (_x_start _x_end _y_start _y_end) (`self.GetTilesAroundPlayerIndices_BP`))
  (bind _queuedtile (`self.QueuedTile`))
  (if (`self.GeneratorBusy`)
    (if (`self.TileDataReady`)
      (`self.DrawTile`))
    (else
      (for _index (range _y_start (+ _y_end 1))
        (for _index_2 (range _x_start (+ _x_end 1))
          (if (not (`.ReturnValue` (`BlueprintMapLibrary.Map_Find` _queuedtile (make `IntPoint` _index_2 _index))))
            (`BlueprintMapLibrary.Map_Add` _queuedtile (make `IntPoint` _index_2 _index) -1) ; queued, but not generated
          )))
      (bind _returnvalue (`self.GetClosestQueuedTile`))
      (if (== (`BlueprintMapLibrary.Map_Find` (`self.QueuedTile`) _returnvalue) -1)
        (bind (_x _y) (break `IntPoint` _returnvalue))
        (`self.GenerateTerrainAsync` _x _y)))))

(fn `Generate Terrain_BP`
  (params (SectionIndex_X :type Integer) (SectionIndex_Y :type Integer))
  (locals (Vertices_local :type "Array of Vector Structure") (UV0_local :type "Array of Vector2D Structure") (Triangles_local :type "Array of Integer") (Offset_local :type "Vector Structure"))
  (bind _cellsize (`self.CellSize`))
  (bind _triangles_local (`local.Triangles_local`))
  (bind _triangles_local_2 (`local.Triangles_local`))
  (bind _meshsectionindex (`self.MeshSectionIndex`))
  (bind (_offset_local_x _offset_local_y) (`KismetMathLibrary.BreakVector` (`local.Offset_local`)))
  (bind _cellsize_2 (`self.CellSize`))
  (bind _returnvalue (/ (`self.CellSize`) 100.0))
  (bind _returnvalue_2 (+ (`self.XVertexCount`) 2))
  (set `local.Offset_local` (`KismetMathLibrary.MakeVector` (`KismetMathLibrary.Conv_IntToDouble` (* (`local.SectionIndex_X`) (* (- (`self.XVertexCount`) 1) _cellsize))) (`KismetMathLibrary.Conv_IntToDouble` (* (`local.SectionIndex_Y`) (* (- (`self.YVertexCount`) 1) _cellsize)))))
  ;[1 0.9575 0.6945] Generate Vertices + UV
  (for _index (range -1 (+ (`self.YVertexCount`) 1))
    (for _index_2 (range -1 (+ (`self.XVertexCount`) 1))
      (bind _returnvalue_3 (+ _offset_local_x (* _index_2 _cellsize_2)))
      (bind _returnvalue_4 (+ _offset_local_y (* _index _cellsize_2)))
      (`KismetArrayLibrary.Array_Add` (`local.Vertices_local`) (`KismetMathLibrary.MakeVector` _returnvalue_3 _returnvalue_4 (`self.GenerateHeight_BP` _returnvalue_3 _returnvalue_4)))
      (`KismetArrayLibrary.Array_Add` (`local.UV0_local`) (`KismetMathLibrary.MakeVector2D` (* _returnvalue (`KismetMathLibrary.Conv_IntToDouble` (+ _index_2 (* (`local.SectionIndex_X`) (- (`self.XVertexCount`) 1))))) (* _returnvalue (`KismetMathLibrary.Conv_IntToDouble` (+ _index (* (`local.SectionIndex_Y`) (- (`self.YVertexCount`) 1)))))))))
  ;[0.6033 1 0.9541] 1st triangle
  (for _index_3 (range (+ (`self.YVertexCount`) 1))
    (for _index_4 (range (+ (`self.XVertexCount`) 1))
      (bind _returnvalue_5 (+ _index_4 (* _index_3 _returnvalue_2)))
      (`KismetArrayLibrary.Array_Add` _triangles_local_2 _returnvalue_5)
      (bind _returnvalue_6 (+ _returnvalue_5 _returnvalue_2))
      (`KismetArrayLibrary.Array_Add` _triangles_local_2 _returnvalue_6)
      (bind _returnvalue_7 (+ _returnvalue_5 1))
      (`KismetArrayLibrary.Array_Add` _triangles_local_2 _returnvalue_7)
      ;[0.4266 1 0.9302] 2nd triangle
      (`KismetArrayLibrary.Array_Add` _triangles_local _returnvalue_6)
      (`KismetArrayLibrary.Array_Add` _triangles_local (+ _returnvalue_6 1))
      (`KismetArrayLibrary.Array_Add` _triangles_local _returnvalue_7)))
  (bind (_out_vertices_local _out_triangles_local _out_normals _out_uv0_local _out_tangents) (`self.GetSubset_BP` (`local.Vertices_local`) (`local.Triangles_local`) (`local.UV0_local`)))
  (`ProceduralMeshComponent.CreateMeshSection_LinearColor` :`self` (`self.TerrainMesh`) :`SectionIndex` _meshsectionindex :`Vertices` _out_vertices_local :`Triangles` _out_triangles_local :`Normals` _out_normals :`UV0` _out_uv0_local :`Tangents` _out_tangents :`bCreateCollision` true)
  (bind _terrainmaterial (`self.TerrainMaterial`)
    (:`then`
      (`PrimitiveComponent.SetMaterial` (`self.TerrainMesh`) _meshsectionindex _terrainmaterial))
    (:`else`
      _))
  (`/Engine/EditorBlueprintResources/StandardMacros.IncrementInt` (`self.MeshSectionIndex`)))

(fn `GenerateHeight_BP`
  (params (X :type "Float (double-precision)") (Y :type "Float (double-precision)"))
  (returns (ReturnValue :type "Float (double-precision)"))
  (return (+ (`self.PerlinNoise2D_BP` X Y 0.0001 10000.0 0.1) (`self.PerlinNoise2D_BP` X Y 0.001 2000.0 0.2) (`self.PerlinNoise2D_BP` X Y 0.002 500.0 0.3))))

(fn `GetPlayerPosIndex_BP`
  (returns (Player_XIndex :type Integer) (Player_YIndex :type Integer))
  (bind _returnvalue (`GameplayStatics.GetPlayerPawn` 0))
  (bind _cellsize (`self.CellSize`))
  (bind (_returnvalue_x _returnvalue_y) (`KismetMathLibrary.BreakVector` (`self.K2_GetActorLocation` _returnvalue)))
  (`/Engine/EditorBlueprintResources/StandardMacros.IsValid` _returnvalue
    (:`Is Valid`
      (return (`KismetMathLibrary.FTrunc` (/ _returnvalue_x (* _cellsize (- (`self.XVertexCount`) 1)))) (`KismetMathLibrary.FTrunc` (/ _returnvalue_y (* _cellsize (- (`self.YVertexCount`) 1))))))
    (:`Is Not Valid`
      (`KismetSystemLibrary.PrintString` "No Valid Player Character -- [Get Player Pos]")
      (return 0 0))))

(fn `GetSubset_BP`
  (params (In_Vertices :type "Array of Vector Structure (by ref)") (In_Triangles :type "Array of Integer (by ref)") (In_UVs :type "Array of Vector2D Structure (by ref)"))
  (returns (Out_Vertices_local :type "Array of Vector Structure") (Out_Triangles_local :type "Array of Integer") (Out_Normals :type "Array of Vector Structure") (Out_UV0_local :type "Array of Vector2D Structure") (Out_Tangents :type "Array of ProcMeshTangent Structure"))
  (locals (Out_Vert :type "Array of Vector Structure") (Out_Tri :type "Array of Integer") (Out_UV :type "Array of Vector2D Structure") (Out_Norm :type "Array of Vector Structure") (Out_Tang :type "Array of ProcMeshTangent Structure") (Big_Normals :type "Array of Vector Structure") (Big_Tangents :type "Array of ProcMeshTangent Structure") (Index :type Integer :default 0))
  (bind _out_tri (`local.Out_Tri`))
  (bind _out_tri_2 (`local.Out_Tri`))
  (bind _xvertexcount (`self.XVertexCount`))
  (bind (_normals _tangents) (`KismetProceduralMeshLibrary.CalculateTangentsForMesh` In_Vertices In_Triangles In_UVs))
  (set `local.Big_Normals` _normals)
  (set `local.Big_Tangents` _tangents)
  (for _index (range -1 (+ (`self.YVertexCount`) 1))
    (for _index_2 (range -1 (+ (`self.XVertexCount`) 1))
      (if (and (> _index_2 -1) (< _index_2 (`self.XVertexCount`)) (> _index -1) (< _index (`self.YVertexCount`)))
        (`KismetArrayLibrary.Array_Add` (`local.Out_Vert`) (`|GetArrayItem` (`local.In_Vertices`) (`local.Index`)))
        (`KismetArrayLibrary.Array_Add` (`local.Out_UV`) (`|GetArrayItem` (`local.In_UVs`) (`local.Index`)))
        (`KismetArrayLibrary.Array_Add` (`local.Out_Norm`) (`|GetArrayItem` (`local.Big_Normals`) (`local.Index`)))
        (`KismetArrayLibrary.Array_Add` (`local.Out_Tang`) (`|GetArrayItem` (`local.Big_Tangents`) (`local.Index`))))
      (`/Engine/EditorBlueprintResources/StandardMacros.IncrementInt` (`local.Index`))))
  (for _index_3 (range (+ (- (`self.YVertexCount`) 2) 1))
    (for _index_4 (range (+ (- (`self.XVertexCount`) 2) 1))
      (bind _returnvalue (+ _index_4 (* _index_3 _xvertexcount)))
      (`KismetArrayLibrary.Array_Add` _out_tri_2 _returnvalue)
      (bind _returnvalue_2 (+ _returnvalue _xvertexcount))
      (`KismetArrayLibrary.Array_Add` _out_tri_2 _returnvalue_2)
      (bind _returnvalue_3 (+ _returnvalue 1))
      (`KismetArrayLibrary.Array_Add` _out_tri_2 _returnvalue_3)
      (`KismetArrayLibrary.Array_Add` _out_tri _returnvalue_2)
      (`KismetArrayLibrary.Array_Add` _out_tri (+ _returnvalue_2 1))
      (`KismetArrayLibrary.Array_Add` _out_tri _returnvalue_3)))
  (return (`local.Out_Vert`) (`local.Out_Tri`) (`local.Out_Norm`) (`local.Out_UV`) (`local.Out_Tang`)))

(fn `GetTilesAroundPlayerIndices_BP`
  (returns (X_start :type Integer) (X_end :type Integer) (Y_start :type Integer) (Y_end :type Integer))
  (bind (_player_xindex _player_yindex) (`self.GetPlayerPosIndex_BP`))
  (bind _numofxsections (`self.NumOfXSections`))
  (bind _numofysections (`self.NumOfYSections`))
  (bind _returnvalue (- _player_yindex (/ _numofysections 2)))
  (bind _returnvalue_2 (- _player_xindex (/ _numofxsections 2)))
  (return _returnvalue_2 (+ _returnvalue_2 _numofxsections -1) _returnvalue (+ _returnvalue _numofysections -1)))

(fn `PerlinNoise2D_BP`
  (params (X :type "Float (double-precision)") (Y :type "Float (double-precision)") (Frequency :type "Float (double-precision)") (Amplitude :type "Float (double-precision)") (Offset :type "Float (double-precision)"))
  (returns (ReturnValue :type "Float (double-precision)"))
  (return (* (* (`KismetMathLibrary.PerlinNoise1D` (+ (* X Frequency) 0.1 Offset)) (`KismetMathLibrary.PerlinNoise1D` (+ (* Y Frequency) 0.1 Offset))) Amplitude)))

(fn `UserConstructionScript`)